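; Test interactable actor that requires a timed interaction, shown by its point light blending from an initial to a final color.
; Begin interact stores the interactor, and Tick accumulates time, updates the light and sends progress messages to the interactor.
; Completion clears the timer and sends an ended message, leaving the light at its reached color.
; Cancel clears the state, restores the initial color and also sends an ended message.
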(event `self.ReceiveBeginPlay`
  (`LightComponent.SetLightColor` (`self.PointLight`) (`self.InitialColor`) true))

(event `self.ReceiveTick`
  (params (DeltaSeconds :type "Float (single-precision)"))
  (bind _interactor (`self.Interactor`))
  (bind _returnvalue (+ (`self.CurrentInteractionDuration`) DeltaSeconds))
  (bind _returnvalue_2 (/ _returnvalue (`self.InteractionDuration`)))
  (if (`self.IsBeingInteracted`)
    (set `self.CurrentInteractionDuration` _returnvalue)
    (`LightComponent.SetLightColor` (`self.PointLight`) (`KismetMathLibrary.LinearColorLerp` (`self.InitialColor`) (`self.FinalColor`) _returnvalue_2) true)
    (if (>= _returnvalue_2 1.0)
      (set `self.IsBeingInteracted` false)
      (set `self.CurrentInteractionDuration` 0.0)
      (message `/Game/Blueprints/Interactability/InteractorInterface.InteractionEnded` _interactor)
      (else
        (message `/Game/Blueprints/Interactability/InteractorInterface.InteractionUpdated` _interactor _returnvalue_2 _interactor)))))

(event `/Game/Blueprints/Interactability/InteractableInterface.OnBeginInteract`
  (params (Interactor :type "Object Object Reference"))
  (set `self.Interactor` Interactor)
  (set `self.IsBeingInteracted` true))

(event `/Game/Blueprints/Interactability/InteractableInterface.OnCancelInteract`
  (params (Interactor :type "Object Object Reference"))
  (set `self.Interactor` null)
  (set `self.IsBeingInteracted` false)
  (set `self.CurrentInteractionDuration` 0.0)
  (`LightComponent.SetLightColor` (`self.PointLight`) (`self.InitialColor`) true)
  (message `/Game/Blueprints/Interactability/InteractorInterface.InteractionEnded` Interactor))

(fn `UserConstructionScript`)