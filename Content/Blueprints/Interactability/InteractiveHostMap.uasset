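; Interactive host map actor that toggles its point light and opens the hosting menu when interacted with.
; On begin interact it flips IsLightOn, applies it to the PointLight visibility, and tells the interactor the interaction ended.
; It then casts player 0's pawn to ThirdPersonCharacter and calls ShowHostingMenu, regardless of who interacted.
; Cancelling an interaction only sends the ended message back to the interactor.
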(event `/Game/Blueprints/Interactability/InteractableInterface.OnBeginInteract`
  (params (Interactor :type "Object Object Reference"))
  (if (`self.IsLightOn`)
    (set `self.IsLightOn` false)
    (else
      (set `self.IsLightOn` true)))
  (`SceneComponent.SetVisibility` (`self.PointLight`) (`self.IsLightOn`) false)
  (message `/Game/Blueprints/Interactability/InteractorInterface.InteractionEnded` Interactor)
  (bind _asthird_person_character (cast `/Game/ThirdPersonCPP/Blueprints/ThirdPersonCharacter` (`GameplayStatics.GetPlayerCharacter` 0)))
  (`/Game/ThirdPersonCPP/Blueprints/ThirdPersonCharacter.ShowHostingMenu` _asthird_person_character))

(event `/Game/Blueprints/Interactability/InteractableInterface.OnCancelInteract`
  (params (Interactor :type "Object Object Reference"))
  (message `/Game/Blueprints/Interactability/InteractorInterface.InteractionEnded` Interactor))

(fn `UserConstructionScript`)