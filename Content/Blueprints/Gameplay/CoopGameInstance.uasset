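; CoopGameInstance is the co-op game's Game Instance, handling network failures.
; On a network error it prints a notice and destroys the first player's session.
; When destruction succeeds, it returns to the MainMenu level and prints a debug message naming the specific failure type.
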(event `self.HandleNetworkError`
  (params (FailureType :type "ENetworkFailure Enum" :default "NetDriverAlreadyExists") (bIsServer :type Boolean))
  (`KismetSystemLibrary.PrintString` "Network failure!")
  (`DestroySessionCallbackProxy.DestroySession` (`GameplayStatics.GetPlayerController` 0)
    (:`then`
      (`GameplayStatics.OpenLevel` "MainMenu")
      (switch `ENetworkFailure` FailureType
        (:`NetDriverAlreadyExists`
          (`KismetSystemLibrary.PrintString` "Net Driver Already Exists"))
        (:`NetDriverCreateFailure`
          (`KismetSystemLibrary.PrintString` "Net Driverr Create Failure"))
        (:`NetDriverListenFailure`
          (`KismetSystemLibrary.PrintString` "Net Driver Listen Failure"))
        (:`ConnectionLost`
          (`KismetSystemLibrary.PrintString` "Connection Lost"))
        (:`ConnectionTimeout`
          (`KismetSystemLibrary.PrintString` "Connection Timeout"))
        (:`FailureReceived`
          (`KismetSystemLibrary.PrintString` "Failure Received"))
        (:`OutdatedClient`
          (`KismetSystemLibrary.PrintString` "Outdated Client"))
        (:`OutdatedServer`
          (`KismetSystemLibrary.PrintString` "Outdated Server"))
        (:`PendingConnectionFailure`
          (`KismetSystemLibrary.PrintString` "Pending Connection Failure"))))))