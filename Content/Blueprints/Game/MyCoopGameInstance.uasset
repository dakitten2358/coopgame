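; Game instance for a co-op game that tracks the high-level game state and shows the main menu.
; BeginPlayShowMainMenu shows the menu only when the current state is Startup.
; The menu event opens a level if leaving Playing (level name is None), then transitions to MainMenu.
; It creates the menu widget once, reuses it, adds it to the viewport, and enables UI-only input with a visible cursor.
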(event `CustomEvent_0`
  (bind _returnvalue (`GameplayStatics.GetPlayerController` 0))
  (if (`self.IsCurrentState` "Playing")
    (`GameplayStatics.OpenLevel` "None"))
  (`self.TransitionToState` "MainMenu")
  (`/Engine/EditorBlueprintResources/StandardMacros.IsValid` (`self.MainMenu`)
    (:`Is Valid`
      _)
    (:`Is Not Valid`
      (bind _returnvalue_2 (`|CreateWidget` "/Game/UI/MainMenu/MainMenu.MainMenu_C" _returnvalue))
      (bind _output_get (set `self.MainMenu` _returnvalue_2))))
  (`WidgetBlueprintLibrary.SetInputMode_UIOnlyEx` _returnvalue _output_get)
  (`UserWidget.AddToViewport` (`self.MainMenu`) 0)
  (set `PlayerController.bShowMouseCursor` true _returnvalue))

(fn `BeginPlay Show Main Menu`
  (if (`self.IsCurrentState` "Startup")
    (`self.ShowMainMenu`)))