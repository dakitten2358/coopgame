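; GameInfoInstance is a game instance Blueprint that owns and displays the main menu and loading screen widgets.
; ShowMainMenu and ShowLoadingScreen each create their widget for the first player controller only if the stored reference is invalid, then add it to the viewport.
; Showing the main menu also turns on the mouse cursor.
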(event `ShowMainMenu`
  (bind _returnvalue (`GameplayStatics.GetPlayerController` 0))
  ;[1 1 1] Create (?) and show main menu
  (`/Engine/EditorBlueprintResources/StandardMacros.IsValid` (`self.MainMenuWidget`)
    (:`Is Valid`
      _)
    (:`Is Not Valid`
      (bind _returnvalue_2 (`|CreateWidget` "/Game/UI/MainMenu/MainMenu.MainMenu_C" _returnvalue))
      (set `self.MainMenuWidget` _returnvalue_2)))
  (`UserWidget.AddToViewport` (`self.MainMenuWidget`) 0)
  (set `PlayerController.bShowMouseCursor` true _returnvalue))

(event `ShowLoadingScreen`
  ;[1 1 1] Show Loading Screen
  (`/Engine/EditorBlueprintResources/StandardMacros.IsValid` (`self.LoadingScreenWidget`)
    (:`Is Valid`
      _)
    (:`Is Not Valid`
      (bind _returnvalue (`|CreateWidget` "/Game/UI/Common/LoadingScreen.LoadingScreen_C" (`GameplayStatics.GetPlayerController` 0)))
      (bind _output_get (set `self.LoadingScreenWidget` _returnvalue))))
  (`UserWidget.AddToViewport` _output_get 0))